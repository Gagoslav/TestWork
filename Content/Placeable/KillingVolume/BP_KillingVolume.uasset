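; BP_KillingVolume is a placeable damage volume that hurts a TestWorkCharacter with a HealthComponent while it overlaps the Box.
; Begin overlap caches the character and starts a looping timer that applies DamageValue every DamageFrequency and prints remaining health.
; The timer clears when health is depleted or any overlap ends.
; Only one character and timer handle are stored, so only the latest entrant is tracked.
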(event `self.Box.OnComponentBeginOverlap`
  (params (OverlappedComponent :type "PrimitiveComponent Object Reference") (OtherActor :type "Actor Object Reference") (OtherComp :type "PrimitiveComponent Object Reference") (OtherBodyIndex :type Integer) (bFromSweep :type Boolean) (SweepResult :type "HitResult Structure (by ref)"))
  (`/Engine/EditorBlueprintResources/StandardMacros.IsValid` (`self.GetComponentByClass` OtherActor "/Script/TestWork.HealthComponent")
    (:`Is Valid`
      (bind _astest_work_character (cast `TestWorkCharacter` OtherActor))
      (bind _output_get (set `self.CachedCharacter` _astest_work_character))
      (bind _returnvalue (`KismetSystemLibrary.K2_SetTimerDelegate` (delegate `ApplyDamage`) (`self.DamageFrequency`) true))
      (set `self.Timer` _returnvalue))))

(event `ApplyDamage`
  (bind _healthcomponent (`TestWorkCharacter.HealthComponent` (stale `self.Box.OnComponentBeginOverlap` _output_get)))
  (bind _health (`HealthComponent.Health` _healthcomponent))
  (if (> _health 0.0)
    (`HealthComponent.ApplyDamage` _healthcomponent (`self.DamageValue`))
    (`KismetSystemLibrary.PrintString` (`KismetStringLibrary.Conv_DoubleToString` _health) true true (struct :`G` 0.66 :`B` 1.0 :`A` 1.0) 0.2)
    (else
      (`KismetSystemLibrary.K2_ClearAndInvalidateTimerHandle` (`self.Timer`)))))

(event `self.Box.OnComponentEndOverlap`
  (params (OverlappedComponent :type "PrimitiveComponent Object Reference") (OtherActor :type "Actor Object Reference") (OtherComp :type "PrimitiveComponent Object Reference") (OtherBodyIndex :type Integer))
  (`KismetSystemLibrary.K2_ClearAndInvalidateTimerHandle` (`self.Timer`)))

(fn `UserConstructionScript`)